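; PC_MainMenu is the main menu player controller, which puts the menu on screen when play begins.
; On BeginPlay it creates W_MainMenu, stores it, adds it to the viewport and shows the mouse cursor on player controller 0.
; When the Steam online subsystem is present, it waits briefly, then passes the player's nickname to the widget, a step marked to move to PlayerState later.
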(event EventBeginPlay
  (bind _returnvalue (Game|GetPlayerController 0))
  (bind _returnvalue_2 (UserInterface|CreateWidget "/Game/_Main/Widgets/W_MainMenu.W_MainMenu_C" _returnvalue))
  (bind _output_get (Variables|Default|SetMainMenuWidget _returnvalue_2))
  (UserInterface|Viewport|AddtoViewport _output_get 0)
  (Variables|/Script/Engine.PlayerController|SetbShowMouseCursor _returnvalue true)
  (if (Class|AdvancedSessionsLibrary|HasOnlineSubsystem "STEAM")
    (Utilities|FlowControl|Delay 0.2)
    (Default|SetPlayerName (Variables|Default|GetMainMenuWidget) (Utilities|Text|ToText(String) (Class|AdvancedIdentityLibrary|GetPlayerNickname (Class|AdvancedSessionsLibrary|GetUniqueNetID (Game|GetPlayerController 0)))))))

(fn ConstructionScript)