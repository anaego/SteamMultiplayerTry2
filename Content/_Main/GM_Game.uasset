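; Game mode for a session-based, two-team multiplayer match that assigns teams and decides the winner.
; PostLogin registers each pawn after a short delay, alternates its team and skin, creates widgets, and keeps input disabled until two players join.
; CheckEndGame sets per-team alive flags from IsDead, each overwritten by that team's last listed player.
; When only one team's flag holds, it sends players the result and destroys the session after a delay.
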(event Custom|CheckEndGame
  ;[1 0.4107 0.2569] TODO to cpp?
  (for _array_element (Variables|Default|GetPlayers)
    (switch Utilities|FlowControl|Switch|SwitchonETeam (Variables|/Script/SteamMultiplayerTry2.MainCharacter|GetTeam _array_element)
      (:TeamA
        (Variables|Default|SetTeamAHasPlayers (not (Variables|/Script/SteamMultiplayerTry2.MainCharacter|GetIsDead _array_element))))
      (:TeamB
        (Variables|Default|SetTeamBHasPlayers (not (Variables|/Script/SteamMultiplayerTry2.MainCharacter|GetIsDead _array_element))))))
  (if (and (Variables|Default|GetTeamAHasPlayers) (not (Variables|Default|GetTeamBHasPlayers))) ; If team A won
    (for _array_element_2 (Variables|Default|GetPlayers)
      (Default|EventEndGame _array_element_2 (Utilities|Enum|Equal(Enum) (Variables|/Script/SteamMultiplayerTry2.MainCharacter|GetTeam _array_element_2) "TeamA")))
    (Utilities|FlowControl|Delay 5.0 :!label _label)
    (bind _asmain_game_instance (Utilities|Casting|CastToMainGameInstance (Game|GetGameInstance)))
    (Default|EventDestroySession _asmain_game_instance)
    (elif (and (Variables|Default|GetTeamBHasPlayers) (not (Variables|Default|GetTeamAHasPlayers))) ; If team B won
      (for _array_element_3 (Variables|Default|GetPlayers)
        (Default|EventEndGame _array_element_3 (Utilities|Enum|Equal(Enum) (Variables|/Script/SteamMultiplayerTry2.MainCharacter|GetTeam _array_element_3) "TeamB")))
      (goto _label))))

(event Custom|UpdatePlayerSkin
  (params (NewPlayer :type Third%20Person%20Character%20Object%20Reference))
  (bind _output_get (Variables|/Script/SteamMultiplayerTry2.MainCharacter|SetTeam NewPlayer (Variables|Default|GetNextPlayerTeam)))
  (switch Utilities|FlowControl|Switch|SwitchonETeam _output_get
    (:TeamA
      (Variables|Default|SetNextPlayerTeam "TeamB"))
    (:TeamB
      (Variables|Default|SetNextPlayerTeam "TeamA")))
  (Utilities|FlowControl|Delay 0.2)
  (Default|EventUpdateTeamSkin NewPlayer))

(event EventBeginPlay)

(event EventTick
  (params (DeltaSeconds :type Float%20%28single-precision%29)))

(event EventPostLogin
  (params (NewPlayer :type Player%20Controller%20Object%20Reference))
  (bind _players (Variables|Default|GetPlayers))
  (bind _aspc_game (Utilities|Casting|CastToPC_Game NewPlayer)
    (:then
      (Utilities|FlowControl|Delay 0.2)
      (bind _asthird_person_character (Utilities|Casting|CastToThirdPersonCharacter (Pawn|GetControlledPawn _aspc_game))
        (:then
          (Utilities|Array|Add (Variables|Default|GetPlayers) _asthird_person_character)
          (CallFunction|UpdatePlayerSkin _asthird_person_character)
          (Default|EventCreateWidgets _asthird_person_character)
          (bind _returnvalue (Class|GameModeBase|GetNumPlayers))
          (if (>= _returnvalue 2)
            (for _array_element _players
              (Default|EventEnableInput _array_element)
              (Default|ChangeInfoText _array_element))
            (else
              (for _array_element_2 _players
                (Default|EventDisableInput _array_element_2)))))
        (:CastFailed
          (Development|PrintString "Cast to ThirdPersonCharacter failed"))))
    (:CastFailed
      (Development|PrintString "Cast to PC_Game failed"))))

(fn ConstructionScript)