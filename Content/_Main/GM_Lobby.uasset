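; Lobby game mode that assigns joining players to alternating teams and triggers the matching skin update.
; PostLogin passes the new PC_Lobby controller to UpdatePlayerSkin, which waits briefly before fetching its ThirdPersonCharacter pawn.
; It sets the pawn's Team from NextPlayerTeam, flips that variable between Team A and Team B, then calls EventUpdateTeamSkin.
; On-screen prints report both team values and any failed casts.
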(event Custom|UpdatePlayerSkin
  (params (NewPlayer :type Player%20Controller%20Object%20Reference))
  (bind _aspc_lobby (Utilities|Casting|CastToPC_Lobby NewPlayer)
    (:then
      (Utilities|FlowControl|Delay 0.2)
      (bind _asthird_person_character (Utilities|Casting|CastToThirdPersonCharacter (Pawn|GetControlledPawn _aspc_lobby))
        (:then
          (bind _output_get (Variables|/Script/SteamMultiplayerTry2.MainCharacter|SetTeam _asthird_person_character (Variables|Default|GetNextPlayerTeam)))
          (switch Utilities|FlowControl|Switch|SwitchonETeam _output_get
            (:TeamA
              (Variables|Default|SetNextPlayerTeam "TeamB"))
            (:TeamB
              (Variables|Default|SetNextPlayerTeam "TeamA")))
          (Default|EventUpdateTeamSkin _asthird_person_character)
          (Development|PrintString (Utilities|String|EnumtoString (Variables|/Script/SteamMultiplayerTry2.MainCharacter|GetTeam _asthird_person_character)) true true "(R=0.007220,G=0.190972,B=0.000000,A=1.000000)" 1e+01)
          (Development|PrintString (Utilities|String|EnumtoString (Variables|Default|GetNextPlayerTeam)) true true "(R=0.482639,G=0.105086,B=0.000000,A=1.000000)" 1e+01))
        (:CastFailed
          (Development|PrintString "Cast to ThirdPersonCharacter failed"))))
    (:CastFailed
      (Development|PrintString "Cast to PC_Lobby failed"))))

(event EventBeginPlay)

(event EventTick
  (params (DeltaSeconds :type Float%20%28single-precision%29)))

(event EventPostLogin
  (params (NewPlayer :type Player%20Controller%20Object%20Reference))
  (CallFunction|UpdatePlayerSkin NewPlayer))

(fn ConstructionScript)